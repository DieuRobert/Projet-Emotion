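; BP_ventDeFace is a headwind volume that affects the player character while it overlaps the Box.
; Entering calls VentDeFaceStart on BP_ThirdPersonCharacter with LaunchVelocityX and leaving calls VentDeFaceStop, so the character handles the push itself.
; The construction script configures the NSVent effect's rates, trail size, colors and random seed offset, deriving sprite lifetime and smoke spawn rate from the actor's scale.
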(event OnComponentBeginOverlap(Box)
  (params (OverlappedComponent :type Primitive%20Component%20Object%20Reference) (OtherActor :type Actor%20Object%20Reference) (OtherComp :type Primitive%20Component%20Object%20Reference) (OtherBodyIndex :type Integer) (bFromSweep :type Boolean) (SweepResult :type Hit%20Result%20Structure%20%28by%20ref%29))
  (bind _returnvalue (Game|GetPlayerCharacter 0))
  (if (== OtherActor _returnvalue)
    (bind _asbp_third_person_character (Utilities|Casting|CastToBP_ThirdPersonCharacter _returnvalue))
    (Default|VentDeFaceStart _asbp_third_person_character (Variables|Default|GetlaunchVelocityX))))

(event OnComponentEndOverlap(Box)
  (params (OverlappedComponent :type Primitive%20Component%20Object%20Reference) (OtherActor :type Actor%20Object%20Reference) (OtherComp :type Primitive%20Component%20Object%20Reference) (OtherBodyIndex :type Integer))
  (bind _returnvalue (Game|GetPlayerCharacter 0))
  (if (== OtherActor _returnvalue)
    (bind _asbp_third_person_character (Utilities|Casting|CastToBP_ThirdPersonCharacter _returnvalue))
    (Default|VentDeFaceStop _asbp_third_person_character)))

(event EventBeginPlay)

(event Collision|EventActorBeginOverlap
  (params (OtherActor :type Actor%20Object%20Reference)))

(event EventTick
  (params (DeltaSeconds :type Float%20%28single-precision%29)))

(fn ConstructionScript
  (bind _returnvalue (Class|Actor|GetActorRelativeScale3D))
  (bind _ns_vent (Variables|Default|GetNS_Vent))
  (Niagara|SetNiagaraVariable(Float) _ns_vent "SpawnRate" (Variables|Default|GetVFX_SpawnRate))
  (Niagara|SetNiagaraVariable(Float) _ns_vent "Trails_Size" (Variables|Default|GetVFX_TrailSize))
  (Niagara|SetNiagaraVariable(Float) _ns_vent "Sprite_Lifetime" (* (.z (Class|Actor|GetActorRelativeScale3D)) 0.15))
  (Class|NiagaraComponent|SetRandomSeedOffset _ns_vent (Math|Random|RandomIntegerinRange 0 100))
  (Niagara|SetNiagaraVariable(LinearColor) _ns_vent "Trails_Color" (Variables|Default|GetTrails_Color))
  (Niagara|SetNiagaraVariable(LinearColor) _ns_vent "SnowFlakes_Color" (Variables|Default|GetSnowFlakes_Color))
  (Niagara|SetNiagaraVariable(Float) _ns_vent "Smoke_SpawnRate" (* (+ (.x _returnvalue) (.y _returnvalue)) 4.0)))