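; BP_socle is a pedestal that snaps grabbable props onto itself and signals a linked auto door.
; On BeginPlay it stores the BP_autoDoor matching its first actor tag.
; When an IN_grab actor overlaps the box, physics turns off and a timeline lerps it above the box with zeroed rotation.
; When the timeline finishes it calls FiAdMessage on the door; ending overlap does nothing.
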(event OnComponentBeginOverlap(Box)
  (params (OverlappedComponent :type Primitive%20Component%20Object%20Reference) (OtherActor :type Actor%20Object%20Reference) (OtherComp :type Primitive%20Component%20Object%20Reference) (OtherBodyIndex :type Integer) (bFromSweep :type Boolean) (SweepResult :type Hit%20Result%20Structure%20%28by%20ref%29))
  (bind _rootcomponent (Variables|/Script/Engine.Actor|GetRootComponent OtherActor))
  (if (Utilities|DoesObjectImplementInterface OtherActor "/Game/Blueprint/DATA/Interfaces/IN_grab.IN_grab_C")
    (Physics|SetSimulatePhysics OtherComp false)
    (bind _newtrack_0 (Timeline|Timeline PlayFromStart)
      (:Update
        (Transformation|SetWorldLocationAndRotation _rootcomponent (Math|Vector|Lerp(Vector) (Transformation|GetWorldLocation _rootcomponent) (+ (Transformation|GetWorldLocation (Variables|Default|GetBox)) "0.000000,0.000000,50.000000") _newtrack_0) (Math|Rotator|Lerp(Rotator) (Transformation|GetWorldRotation _rootcomponent) "0, 0, 0" _newtrack_0) false false))
      (:Finished
        (Class|IAD|FiAd(Message) (Variables|Default|Getdoor))))))

(event OnComponentEndOverlap(Box)
  (params (OverlappedComponent :type Primitive%20Component%20Object%20Reference) (OtherActor :type Actor%20Object%20Reference) (OtherComp :type Primitive%20Component%20Object%20Reference) (OtherBodyIndex :type Integer))
  (if (Utilities|DoesObjectImplementInterface OtherActor "/Game/Blueprint/DATA/Interfaces/IN_grab.IN_grab_C")
    _))

(event EventBeginPlay
  (bind _outactors (Actor|GetAllActorsOfClasswithTag "/Game/Blueprint/Props/grab/BP_autoDoor.BP_autoDoor_C" (Utilities|Array|Get(acopy) (Variables|Actor|GetTags))))
  (for _array_element _outactors
    (Variables|Default|Setdoor _array_element)))

(fn ConstructionScript)