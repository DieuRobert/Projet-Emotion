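; BP_Zones is a trigger volume that tells the third-person character which zone it has entered.
; On BeginPlay it caches the first BP_ThirdPersonCharacter found in the level.
; When that character begins overlapping the Box component, it copies its ZoneBox value into the character's ZoneTPC and prints the result for debugging.
; There is no end-overlap handling, so this actor never clears the value on exit.
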(event OnComponentBeginOverlap(Box)
  (params (OverlappedComponent :type Primitive%20Component%20Object%20Reference) (OtherActor :type Actor%20Object%20Reference) (OtherComp :type Primitive%20Component%20Object%20Reference) (OtherBodyIndex :type Integer) (bFromSweep :type Boolean) (SweepResult :type Hit%20Result%20Structure%20%28by%20ref%29))
  (bind _bp_thirdpersoncharacter (Variables|Default|GetBP_ThirdPersonCharacter))
  (if (== OtherActor _bp_thirdpersoncharacter)
    (bind _output_get (Variables|/Game/ThirdPerson/Blueprints/BP_ThirdPersonCharacter.BP_ThirdPersonCharacter_C|SetzoneTPC _bp_thirdpersoncharacter (Variables|Default|GetzoneBox)))
    (Development|PrintString (Utilities|String|ToString(Name) _output_get))))

(event EventBeginPlay
  (bind _outactors (Actor|GetAllActorsOfClass "/Game/ThirdPerson/Blueprints/BP_ThirdPersonCharacter.BP_ThirdPersonCharacter_C"))
  (Variables|Default|SetBP_ThirdPersonCharacter (Utilities|Array|Get(acopy) _outactors)))

(fn ConstructionScript)