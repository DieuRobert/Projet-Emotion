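; BP_cameraLow is a trigger volume that changes the third-person camera's pitch while the player character is inside its Box.
; Overlap begin plays the AbsoluteRotationStart timeline, whose Y value drives the pitch of the character's SpringArm in world rotation, with roll and yaw held at zero.
; Overlap end reverses the same timeline to transition the angle back.
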(event OnComponentBeginOverlap(Box)
  (params (OverlappedComponent :type Primitive%20Component%20Object%20Reference) (OtherActor :type Actor%20Object%20Reference) (OtherComp :type Primitive%20Component%20Object%20Reference) (OtherBodyIndex :type Integer) (bFromSweep :type Boolean) (SweepResult :type Hit%20Result%20Structure%20%28by%20ref%29))
  (bind _returnvalue (Game|GetPlayerCharacter 0))
  (if (== OtherActor _returnvalue)
    (bind _asbp_third_person_character (Utilities|Casting|CastToBP_ThirdPersonCharacter _returnvalue))
    (bind _y (Timeline|absoluteRotationStart Play)
      (:Update
        (Transformation|SetWorldRotation (Variables|/Game/ThirdPerson/Blueprints/BP_ThirdPersonCharacter.BP_ThirdPersonCharacter_C|GetSpringArm _asbp_third_person_character) (Math|Rotator|MakeRotator 0.0 _y 0.0) false false)))))

(event OnComponentEndOverlap(Box)
  (params (OverlappedComponent :type Primitive%20Component%20Object%20Reference) (OtherActor :type Actor%20Object%20Reference) (OtherComp :type Primitive%20Component%20Object%20Reference) (OtherBodyIndex :type Integer))
  (if (== OtherActor (Game|GetPlayerCharacter 0))
    (bind _y (Timeline|absoluteRotationStart Reverse)
      (:Update
        (Transformation|SetWorldRotation (Variables|/Game/ThirdPerson/Blueprints/BP_ThirdPersonCharacter.BP_ThirdPersonCharacter_C|GetSpringArm (stale OnComponentBeginOverlap(Box) _asbp_third_person_character)) (Math|Rotator|MakeRotator 0.0 _y 0.0) false false)))))

(fn ConstructionScript)