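; BP_cameraChangeRotation is a trigger box that swings the third-person camera to a new yaw when the player character overlaps it.
; On overlap it stores the spring arm's current world yaw and plays a timeline.
; Each update blends the arm's yaw from that value to CamEndRot, keeping pitch and roll.
; It also feeds a CamStartYaw-to-CamEndYaw blend into AddControllerYawInput as per-update input, not an absolute angle.
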(event OnComponentBeginOverlap(Box)
  (params (OverlappedComponent :type Primitive%20Component%20Object%20Reference) (OtherActor :type Actor%20Object%20Reference) (OtherComp :type Primitive%20Component%20Object%20Reference) (OtherBodyIndex :type Integer) (bFromSweep :type Boolean) (SweepResult :type Hit%20Result%20Structure%20%28by%20ref%29))
  (bind _returnvalue (Game|GetPlayerCharacter 0))
  (if (== OtherActor _returnvalue)
    (bind _asbp_third_person_character (Utilities|Casting|CastToBP_ThirdPersonCharacter _returnvalue))
    (bind _output_get (Variables|Default|SetReturn%20Value%20Z%20%28Yaw%29 (.yaw (Transformation|GetWorldRotation (Variables|/Game/ThirdPerson/Blueprints/BP_ThirdPersonCharacter.BP_ThirdPersonCharacter_C|GetSpringArm _asbp_third_person_character)))))
    (bind _rot (Timeline|Timeline Play)
      (:Update
        (Pawn|Input|AddControllerYawInput _asbp_third_person_character (Math|Float|Lerp (Variables|Default|GetcamStartYaw) (Variables|Default|GetcamEndYaw) _rot))
        (Transformation|SetWorldRotation (Variables|/Game/ThirdPerson/Blueprints/BP_ThirdPersonCharacter.BP_ThirdPersonCharacter_C|GetSpringArm _asbp_third_person_character) (Math|Rotator|MakeRotator (.roll (Transformation|GetWorldRotation (Variables|/Game/ThirdPerson/Blueprints/BP_ThirdPersonCharacter.BP_ThirdPersonCharacter_C|GetSpringArm _asbp_third_person_character))) (.pitch (Transformation|GetWorldRotation (Variables|/Game/ThirdPerson/Blueprints/BP_ThirdPersonCharacter.BP_ThirdPersonCharacter_C|GetSpringArm _asbp_third_person_character))) (Math|Float|Lerp _output_get (Variables|Default|GetcamEndRot) _rot)) false false)))))

(fn ConstructionScript)