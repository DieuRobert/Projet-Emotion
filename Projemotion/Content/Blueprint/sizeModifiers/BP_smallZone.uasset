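; BP_smallZone is a trigger zone that permits the third-person character to shrink while inside it.
; On BeginPlay it caches the first BP_ThirdPersonCharacter found in the level and responds only to that actor's overlaps with its Box.
; Entering sets the character's CanRapetisser flag; leaving clears it and resets the capsule's world scale to normal.
; The zone performs no shrinking itself.
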(event OnComponentBeginOverlap(Box)
  (params (OverlappedComponent :type Primitive%20Component%20Object%20Reference) (OtherActor :type Actor%20Object%20Reference) (OtherComp :type Primitive%20Component%20Object%20Reference) (OtherBodyIndex :type Integer) (bFromSweep :type Boolean) (SweepResult :type Hit%20Result%20Structure%20%28by%20ref%29))
  (bind _bp_thirdpersoncharacter (Variables|Default|GetBP_ThirdPersonCharacter))
  (if (== OtherActor _bp_thirdpersoncharacter)
    (Variables|/Game/ThirdPerson/Blueprints/BP_ThirdPersonCharacter.BP_ThirdPersonCharacter_C|SetcanRapetisser _bp_thirdpersoncharacter true)))

(event OnComponentEndOverlap(Box)
  (params (OverlappedComponent :type Primitive%20Component%20Object%20Reference) (OtherActor :type Actor%20Object%20Reference) (OtherComp :type Primitive%20Component%20Object%20Reference) (OtherBodyIndex :type Integer))
  (bind _bp_thirdpersoncharacter (Variables|Default|GetBP_ThirdPersonCharacter))
  (if (== OtherActor _bp_thirdpersoncharacter)
    (Variables|/Game/ThirdPerson/Blueprints/BP_ThirdPersonCharacter.BP_ThirdPersonCharacter_C|SetcanRapetisser _bp_thirdpersoncharacter false)
    (Transformation|SetWorldScale3D (Variables|/Script/Engine.Character|GetCapsuleComponent _bp_thirdpersoncharacter) "1.000000,1.000000,1.000000")))

(event EventBeginPlay
  (bind _outactors (Actor|GetAllActorsOfClass "/Game/ThirdPerson/Blueprints/BP_ThirdPersonCharacter.BP_ThirdPersonCharacter_C"))
  (Variables|Default|SetBP_ThirdPersonCharacter (Utilities|Array|Get(acopy) _outactors)))

(fn ConstructionScript)