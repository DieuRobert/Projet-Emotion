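; BP_tuto_Glide is a trigger actor that switches the player character's glide ability on or off.
; On BeginPlay it waits briefly, then retries the cast to BP_ThirdPersonCharacter every second until it can cache the reference.
; When the player overlaps the actor, it copies its ActivateGlide value into the character's CanGlide flag.
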(event EventBeginPlay
  (Utilities|FlowControl|Delay 0.2)
  (bind _asbp_third_person_character (Utilities|Casting|CastToBP_ThirdPersonCharacter (Game|GetPlayerCharacter 0) :!label _label)
    (:then
      (Variables|Default|SetPlayerCharacter _asbp_third_person_character))
    (:CastFailed
      (Utilities|FlowControl|Delay 1.0)
      (goto _label))))

(event Collision|EventActorBeginOverlap
  (params (OtherActor :type Actor%20Object%20Reference))
  (if (== OtherActor (Game|GetPlayerCharacter 0))
    (Variables|/Game/ThirdPerson/Blueprints/BP_ThirdPersonCharacter.BP_ThirdPersonCharacter_C|SetcanGlide (Variables|Default|GetPlayerCharacter) (Variables|Default|GetActivateGlide?))))

(fn ConstructionScript)