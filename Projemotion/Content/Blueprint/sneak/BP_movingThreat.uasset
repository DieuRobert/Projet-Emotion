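; BP_movingThreat is a rotating sentry actor, apparently for a sneak mechanic, that watches for the player with PawnSensing.
; From BeginPlay, a Timeline adds its Z value to the root's local yaw on each update and restarts itself when finished.
; Seeing the player character only prints a debug "Hello", and a SetActorRotation node is left unconnected.
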(event OnSeePawn(PawnSensing)
  (params (Pawn :type Pawn%20Object%20Reference))
  (if (== Pawn (Game|GetPlayerCharacter 0))
    (Development|PrintString "Hello")))

(event Custom|rotationUpdate
  (bind _z (Timeline|Timeline PlayFromStart)
    (:Update
      (Transformation|AddLocalRotation (Variables|Default|GetDefaultSceneRoot self) (Math|Rotator|MakeRotator 0.0 0.0 _z) false false))
    (:Finished
      (CallFunction|RotationUpdate))))

(event EventBeginPlay
  (CallFunction|RotationUpdate))

(fn ConstructionScript)