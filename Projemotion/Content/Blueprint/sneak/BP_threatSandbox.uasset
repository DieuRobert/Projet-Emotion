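; BP_threatSandbox is a moving threat actor that detects the player, apparently a test piece for sneaking.
; A looping Timeline started on BeginPlay drives the root's world X and Y at a fixed Z, replaying itself when finished.
; A sphere overlap with the player character only prints a "FOUND" debug message.
; A stop event halts the Timeline and with it the movement.
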(event OnComponentBeginOverlap(Sphere)
  (params (OverlappedComponent :type Primitive%20Component%20Object%20Reference) (OtherActor :type Actor%20Object%20Reference) (OtherComp :type Primitive%20Component%20Object%20Reference) (OtherBodyIndex :type Integer) (bFromSweep :type Boolean) (SweepResult :type Hit%20Result%20Structure%20%28by%20ref%29))
  (if (== OtherActor (Game|GetPlayerCharacter 0))
    (Development|PrintString "FOUND")))

(event Custom|locationUpdate
  (bind (_direction _x _y) (Timeline|Timeline PlayFromStart)
    (:Update
      (Transformation|SetWorldLocation (Variables|Default|GetDefaultSceneRoot) (Math|Vector|MakeVector _x _y -0.499913) false false))
    (:Finished
      (CallFunction|LocationUpdate))))

(event Custom|stop
  (bind (_direction _x _y) (Timeline|Timeline Stop)
    (:Update
      (Transformation|SetWorldLocation (Variables|Default|GetDefaultSceneRoot) (Math|Vector|MakeVector _x _y -0.499913) false false))
    (:Finished
      (CallFunction|LocationUpdate))))

(event EventBeginPlay
  (CallFunction|LocationUpdate))

(fn ConstructionScript)