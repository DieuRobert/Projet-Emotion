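; BP_threat is a patrolling hazard for a sneak section that catches the player and teleports them to a fixed location.
; A Timeline drives the root along X at fixed world Y and Z, restarting itself on finish until the stop event halts it.
; When the player overlaps its Sphere while the character's Hidden flag is false, it prints "FOUND" and moves the player's capsule to hard-coded coordinates.
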(event OnComponentBeginOverlap(Sphere)
  (params (OverlappedComponent :type Primitive%20Component%20Object%20Reference) (OtherActor :type Actor%20Object%20Reference) (OtherComp :type Primitive%20Component%20Object%20Reference) (OtherBodyIndex :type Integer) (bFromSweep :type Boolean) (SweepResult :type Hit%20Result%20Structure%20%28by%20ref%29))
  (bind _bp_thirdpersoncharacter (Variables|Default|GetBP_ThirdPersonCharacter))
  (if (== OtherActor (Game|GetPlayerCharacter 0))
    (if (not (Variables|/Game/ThirdPerson/Blueprints/BP_ThirdPersonCharacter.BP_ThirdPersonCharacter_C|Gethidden _bp_thirdpersoncharacter))
      (Development|PrintString "FOUND")
      (Transformation|SetWorldLocation (Variables|/Script/Engine.Character|GetCapsuleComponent _bp_thirdpersoncharacter) "-442.157926,8551.746897,-0.499951" false false))))

(event Custom|locationUpdate
  (bind _location (Timeline|Timeline PlayFromStart)
    (:Update
      (Transformation|SetWorldLocation (Variables|Default|GetDefaultSceneRoot) (Math|Vector|MakeVector _location 8994.470796 -0.500034) false false))
    (:Finished
      (CallFunction|LocationUpdate))))

(event Custom|stop
  (bind _location (Timeline|Timeline Stop)
    (:Update
      (Transformation|SetWorldLocation (Variables|Default|GetDefaultSceneRoot) (Math|Vector|MakeVector _location 8994.470796 -0.500034) false false))
    (:Finished
      (CallFunction|LocationUpdate))))

(event EventBeginPlay
  (bind _outactors (Actor|GetAllActorsOfClass "/Game/ThirdPerson/Blueprints/BP_ThirdPersonCharacter.BP_ThirdPersonCharacter_C"))
  (Variables|Default|SetBP_ThirdPersonCharacter (Utilities|Array|Get(acopy) _outactors))
  (CallFunction|LocationUpdate))

(fn ConstructionScript)