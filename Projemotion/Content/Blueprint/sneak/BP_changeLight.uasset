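; Trigger-box actor in the sneak folder, apparently meant to switch lighting between day and night.
; BeginPlay stores a Directional Light from the level in DL, keeping the last one found.
; When the player leaves the box, it calls SetActorRotation with no computed angle and clears the Day flag.
; Begin overlap only checks for the player, and the lerped-pitch logic that would restore Day is disconnected.
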(event OnComponentEndOverlap(Box)
  (params (OverlappedComponent :type Primitive%20Component%20Object%20Reference) (OtherActor :type Actor%20Object%20Reference) (OtherComp :type Primitive%20Component%20Object%20Reference) (OtherBodyIndex :type Integer))
  (if (== (Game|GetPlayerCharacter 0) OtherActor)
    (Transformation|SetActorRotation (Math|Rotator|MakeRotator 0.0 0.0 0.0))
    (Variables|Default|Setday false)))

(event OnComponentBeginOverlap(Box)
  (params (OverlappedComponent :type Primitive%20Component%20Object%20Reference) (OtherActor :type Actor%20Object%20Reference) (OtherComp :type Primitive%20Component%20Object%20Reference) (OtherBodyIndex :type Integer) (bFromSweep :type Boolean) (SweepResult :type Hit%20Result%20Structure%20%28by%20ref%29))
  (if (== OtherActor (Game|GetPlayerCharacter 0))
    _))

(event EventBeginPlay
  (bind _outactors (Actor|GetAllActorsOfClass "/Script/Engine.DirectionalLight"))
  (for _array_element _outactors
    (Variables|Default|SetDL _array_element)))

(fn ConstructionScript)